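; BP_Pawn is a player-controlled camera pawn for viewing and navigating a scene with mouse and keyboard.
; Enhanced Input drives yaw-relative WASD movement and wheel zoom via spring arm length.
; Holding left mouse rotates the control rotation with clamped pitch, while holding right mouse drags the pawn along yaw-aligned axes.
; A left click without cursor movement line-traces from the mouse and moves the pawn to the hit XY, keeping its height.
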(event Input|EnhancedActionEvents|EnhancedInputActionIA_ControlView
  (params (ActionValue :type Float%20%28double-precision%29) (ElapsedSeconds :type Float%20%28double-precision%29) (TriggeredSeconds :type Float%20%28double-precision%29) (InputAction :type Input%20Action%20Object%20Reference :default "/Game/BluePrint/Input/IA_ControlView.IA_ControlView"))
  (bind _springarm (Variables|Default|GetSpringArm))
  ;[0 0 0] 鼠标滚轮控制弹簧臂伸缩
  (:Triggered
    (Variables|/Script/Engine.SpringArmComponent|SetTargetArmLength _springarm (+ (Variables|/Script/Engine.SpringArmComponent|GetTargetArmLength _springarm) (* ActionValue (Variables|Default|GetViewRate))))))

(event Input|EnhancedActionEvents|EnhancedInputActionIA_MyForwardMove
  (params (ActionValue :type Float%20%28double-precision%29) (ElapsedSeconds :type Float%20%28double-precision%29) (TriggeredSeconds :type Float%20%28double-precision%29) (InputAction :type Input%20Action%20Object%20Reference :default "/Game/BluePrint/Input/IA_MyForwardMove.IA_MyForwardMove"))
  ;[0 0 0] WASD控制前后左右移动
  (:Triggered
    (Pawn|Input|AddMovementInput (Math|Vector|GetForwardVector (Math|Rotator|MakeRotator 0.0 0.0 (.yaw (Pawn|GetControlRotation :!class /Script/Engine.Pawn)))) ActionValue false)))

(event Input|EnhancedActionEvents|EnhancedInputActionIA_MyRightMove
  (params (ActionValue :type Float%20%28double-precision%29) (ElapsedSeconds :type Float%20%28double-precision%29) (TriggeredSeconds :type Float%20%28double-precision%29) (InputAction :type Input%20Action%20Object%20Reference :default "/Game/BluePrint/Input/IA_MyRightMove.IA_MyRightMove"))
  ;[0 0 0] WASD控制前后左右移动
  (:Triggered
    (Pawn|Input|AddMovementInput (Math|Vector|GetRightVector (Math|Rotator|MakeRotator 0.0 0.0 (.yaw (Pawn|GetControlRotation :!class /Script/Engine.Pawn)))) ActionValue false)))

(event Input|EnhancedActionEvents|EnhancedInputActionIA_MyRightLook
  (params (ActionValue :type Float%20%28double-precision%29) (ElapsedSeconds :type Float%20%28double-precision%29) (TriggeredSeconds :type Float%20%28double-precision%29) (InputAction :type Input%20Action%20Object%20Reference :default "/Game/BluePrint/Input/IA_MyRightLook.IA_MyRightLook"))
  (bind _returnvalue (Pawn|GetControlRotation :!class /Script/Engine.Pawn))
  ;[1 1 1] 按住鼠标左键进行旋转,按住鼠标右键进行拖拽
  ;;[0 0 0] 左右旋转观看
  (:Triggered
    (if (Variables|Default|GetbIsHoldLeftMouseButton?)
      (Pawn|SetControlRotation (Game|GetPlayerController 0) (Math|Rotator|MakeRotator (.roll _returnvalue) (.pitch _returnvalue) (+ (.yaw _returnvalue) (* ActionValue (Variables|Default|GetRotatorRate)))))
      (else
        ;;[0 0 0] 左右拖拽
        (if (Variables|Default|GetbIsHoldRightMouseButton?)
          (Transformation|SetActorLocation (+ (* (Math|Vector|GetRightVector (Math|Rotator|MakeRotator 0.0 0.0 (.yaw (Pawn|GetControlRotation :!class /Script/Engine.Pawn)))) (* ActionValue (Variables|Default|GetMoveRate))) (Transformation|GetActorLocation)) false false))))))

(event Input|EnhancedActionEvents|EnhancedInputActionIA_MyUpLook
  (params (ActionValue :type Float%20%28double-precision%29) (ElapsedSeconds :type Float%20%28double-precision%29) (TriggeredSeconds :type Float%20%28double-precision%29) (InputAction :type Input%20Action%20Object%20Reference :default "/Game/BluePrint/Input/IA_MyUpLook.IA_MyUpLook"))
  (bind _returnvalue (Pawn|GetControlRotation :!class /Script/Engine.Pawn))
  ;[1 1 1] 按住鼠标左键进行旋转,按住鼠标右键进行拖拽
  ;;[0 0 0] 上下旋转观看
  (:Triggered
    (if (Variables|Default|GetbIsHoldLeftMouseButton?)
      (Pawn|SetControlRotation (Game|GetPlayerController 0) (Math|Rotator|MakeRotator (.roll _returnvalue) (Math|Float|ClampAngle (+ (.pitch _returnvalue) (* ActionValue (Variables|Default|GetRotatorRate))) -7e+01 15.0) (.yaw _returnvalue)))
      (else
        ;;[0 0 0] 前后拖拽
        (if (Variables|Default|GetbIsHoldRightMouseButton?)
          (Transformation|SetActorLocation (+ (* (Math|Vector|GetForwardVector (Math|Rotator|MakeRotator 0.0 0.0 (.yaw (Pawn|GetControlRotation :!class /Script/Engine.Pawn)))) (* ActionValue (Variables|Default|GetMoveRate))) (Transformation|GetActorLocation)) false false))))))

(event EventBeginPlay
  (bind _returnvalue (Game|GetPlayerController 0))
  (bind _returnvalue_2 (PlayerController|LocalPlayerSubsystems|GetEnhancedInputLocalPlayerSubsystem _returnvalue))
  ;[1 0 0] 添加映射上下文
  (Utilities|IsValid _returnvalue_2
    (:Is%20Valid
      (Input|AddMappingContext _returnvalue_2 "/Game/BluePrint/Input/IMP_Base.IMP_Base" 0 "(bIgnoreAllPressedKeysUntilRelease=True,bForceImmediately=False)"))))

(event Input|MouseEvents|LeftMouseButton
  (params (Key :type Key%20Structure :default "None"))
  ;[1 1 1] 按住鼠标左键进行旋转,按住鼠标右键进行拖拽
  ;;[0 0 0] 按下鼠标左(右)键为真,松开为假
  (:Pressed
    (Variables|Default|SetbIsHoldLeftMouseButton? true))
  (:Released
    (Variables|Default|SetbIsHoldLeftMouseButton? false)))

(event Input|MouseEvents|RightMouseButton
  (params (Key :type Key%20Structure :default "None"))
  ;[1 1 1] 按住鼠标左键进行旋转,按住鼠标右键进行拖拽
  ;;[0 0 0] 按下鼠标左(右)键为真,松开为假
  (:Pressed
    (Variables|Default|SetbIsHoldRightMouseButton? true))
  (:Released
    (Variables|Default|SetbIsHoldRightMouseButton? false)))

(event Input|MouseEvents|LeftMouseButton
  (params (Key :type Key%20Structure :default "None"))
  (bind _returnvalue (Game|GetPlayerController 0))
  (bind (_worldlocation _worlddirection) (Game|Player|ConvertMouseLocationToWorldSpace _returnvalue))
  ;[0 0 0] 通过射线检测获取到击中点位位置信息,在设置Actor
  (:Pressed
    (bind _returnvalue_2 (Class|WidgetLayoutLibrary|GetMousePositiononViewport)))
  (:Released
    (bind _returnvalue_3 (Class|WidgetLayoutLibrary|GetMousePositiononViewport))
    (if (Utilities|Operators|EqualEqual _returnvalue_2 _returnvalue_3 0.0001)
      (bind (_outhit _returnvalue_4) (Collision|LineTraceByChannel _worldlocation (+ _worldlocation (* _worlddirection 1e+04)) "TraceTypeQuery1" false 0 "Persistent"))
      (if _returnvalue_4
        (Transformation|SetActorLocation (Math|Vector|MakeVector (.X (Math|Vector|BreakVector (.Location (Collision|BreakHitResult _outhit)))) (.Y (Math|Vector|BreakVector (.Location (Collision|BreakHitResult _outhit)))) (.z (Transformation|GetActorLocation))) false false)))))

(fn ConstructionScript)